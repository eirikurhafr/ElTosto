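; BP_Item_Prop is a destructible prop that breaks apart and awards the player score when touched or damaged.
; Component overlap, actor overlap and any damage all share one path that applies heavy radius damage to its destructible component, then calls GivePlayerScore.
; The hurt origin always reads the damage causer's location, which only the damage event supplies, and no guard prevents repeated scoring.
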(event OnComponentBeginOverlap(Destructible_0)
  (params (OverlappedComponent :type Primitive%20Component%20Object%20Reference) (OtherActor :type Actor%20Object%20Reference) (OtherComp :type Primitive%20Component%20Object%20Reference) (OtherBodyIndex :type Integer) (bFromSweep :type Boolean) (SweepResult :type Hit%20Result%20Structure%20%28by%20ref%29))
  (Class|DestructibleComponent|ApplyRadiusDamage (Variables|Default|GetDestructible_0) 1e+03 (Transformation|GetActorLocation (stale Game|Damage|EventAnyDamage DamageCauser)) 1e+03 1.0 false)
  (CallFunction|GivePlayerScore))

(event EventBeginPlay
  (|CallParentFunction) ; This node is disabled and will not be called.\nDrag off pins to build functionality.
)

(event Collision|EventActorBeginOverlap
  (params (OtherActor :type Actor%20Object%20Reference))
  (Class|DestructibleComponent|ApplyRadiusDamage (Variables|Default|GetDestructible_0) 1e+03 (Transformation|GetActorLocation (stale Game|Damage|EventAnyDamage DamageCauser)) 1e+03 1.0 false)
  (CallFunction|GivePlayerScore))

(event EventTick
  (params (DeltaSeconds :type Float%20%28single-precision%29))
  (|CallParentFunction DeltaSeconds))

(event Game|Damage|EventAnyDamage
  (params (Damage :type Float%20%28single-precision%29) (DamageType :type Damage%20Type%20Object%20Reference) (InstigatedBy :type Controller%20Object%20Reference) (DamageCauser :type Actor%20Object%20Reference))
  (Class|DestructibleComponent|ApplyRadiusDamage (Variables|Default|GetDestructible_0) 1e+03 (Transformation|GetActorLocation DamageCauser) 1e+03 1.0 false)
  (CallFunction|GivePlayerScore))

(fn ConstructionScript
  (|CallParentFunction))