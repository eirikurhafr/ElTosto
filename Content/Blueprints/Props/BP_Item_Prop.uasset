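; BP_Item_Prop is a prop item that gives the player score when it gets moved.
; Each tick it runs the parent tick, then checks whether its StaticMesh component's velocity exceeds a small threshold.
; A DoOnce gate calls GivePlayerScore once per burst of movement and resets when the speed drops back to the threshold or below.
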(event EventBeginPlay
  (|CallParentFunction) ; This node is disabled and will not be called.\nDrag off pins to build functionality.
)

(event Collision|EventActorBeginOverlap
  (params (OtherActor :type Actor%20Object%20Reference)))

(event EventTick
  (params (DeltaSeconds :type Float%20%28single-precision%29))
  (|CallParentFunction DeltaSeconds)
  (if (> (Math|Vector|VectorLength (Transformation|GetComponentVelocity (Variables|Default|GetStaticMesh))) 1e+01)
    (Utilities|FlowControl|DoOnce false :!label _label
      (:Completed
        (CallFunction|GivePlayerScore)))
    (else
      (goto _label Reset))))

(fn ConstructionScript
  (|CallParentFunction))