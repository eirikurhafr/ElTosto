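; Ending-sequence pawn that takes player possession, plays the end song and shows the results widget with the mouse cursor.
; StartEnding fills the widget from BPC_ElTosto's final time and score, adding a time-based bonus.
; Gudni loops random slot animations with padded delays, though the delay re-rolls its key, so it may not match the playing animation.
; Paired timelines loop arm-rotation clapping; StartShaking chains two more timelines without update logic.
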(event Custom|StartPlayingAnim
  (bind _animations (Variables|Default|GetAnimations))
  (bind _keys (Utilities|Map|Keys _animations))
  (Class|AnimInstance|PlaySlotAnimation (Components|SkeletalMesh|GetAnimInstance (Variables|Default|GetGudni)) (Utilities|Array|Get(acopy) _keys (Math|Random|RandomIntegerinRange 0 (- (Utilities|Array|Length _keys) 1))) "DefaultSlot" 0.25 0.25 1.0 1)
  (Utilities|FlowControl|Delay (+ (.Value (Utilities|Map|Find _animations (Utilities|Array|Get(acopy) _keys (Math|Random|RandomIntegerinRange 0 (- (Utilities|Array|Length _keys) 1))))) (Math|Random|RandomFloatinRange 1.0 3.0)))
  (CallFunction|StartPlayingAnim))

(event Custom|StartClapping
  (bind _alpha (Timeline|MoveForward PlayFromStart)
    (:Update
      (Transformation|SetWorldRotation (Variables|Default|GetArmLeft_S) (Math|Rotator|Lerp(Rotator) (Variables|Default|GetNormalRotation) (Variables|Default|GetLeftClapRotation) _alpha true) false false)
      (Transformation|SetWorldRotation (Variables|Default|GetArmRight_S) (Math|Rotator|Lerp(Rotator) (Variables|Default|GetNormalRotation) (Variables|Default|GetRightClapRotation) _alpha true) false false))
    (:Finished
      (bind _alpha_2 (Timeline|MoveBackward PlayFromStart)
        (:Update
          (Transformation|SetWorldRotation (Variables|Default|GetArmLeft_S) (Math|Rotator|Lerp(Rotator) (Variables|Default|GetLeftClapRotation) (Variables|Default|GetNormalRotation) _alpha_2 true) false false)
          (Transformation|SetWorldRotation (Variables|Default|GetArmRight_S) (Math|Rotator|Lerp(Rotator) (Variables|Default|GetRightClapRotation) (Variables|Default|GetNormalRotation) _alpha_2 true) false false))
        (:Finished
          (CallFunction|StartClapping))))))

(event Custom|StartShaking
  (Timeline|Shake Play
    (:Finished
      (Timeline|GoBack Play))))

(event Custom|StartEnding
  (bind _returnvalue (Game|GetPlayerController 0))
  (Pawn|UnPossess _returnvalue)
  (Pawn|Possess _returnvalue self)
  (CallFunction|StartPlayingAnim)
  (CallFunction|StartClapping)
  (bind _returnvalue_2 (UserInterface|CreateWidget "/Game/Blueprints/Ending/Widget_Ending.Widget_Ending_C" _returnvalue))
  (bind _asbpc_el_tosto (Utilities|Casting|CastToBPC_ElTosto _returnvalue))
  (Default|FillinNumbers _returnvalue_2 (Variables|/Game/Blueprints/ElTosto/BPC_ElTosto.BPC_ElTosto_C|GetFinalTime _asbpc_el_tosto) (Variables|/Game/Blueprints/ElTosto/BPC_ElTosto.BPC_ElTosto_C|GetFinalScore _asbpc_el_tosto) (* (Math|Conversions|ToFloat(Integer) (Math|Float|Truncate (/ 2e+01 (Variables|/Game/Blueprints/ElTosto/BPC_ElTosto.BPC_ElTosto_C|GetFinalTime _asbpc_el_tosto)))) (Variables|/Game/Blueprints/ElTosto/BPC_ElTosto.BPC_ElTosto_C|GetFinalScore _asbpc_el_tosto)) (Math|Conversions|ToFloat(Integer) (Math|Float|Truncate (+ (* (Math|Conversions|ToFloat(Integer) (Math|Float|Truncate (/ 2e+01 (Variables|/Game/Blueprints/ElTosto/BPC_ElTosto.BPC_ElTosto_C|GetFinalTime _asbpc_el_tosto)))) (Variables|/Game/Blueprints/ElTosto/BPC_ElTosto.BPC_ElTosto_C|GetFinalScore _asbpc_el_tosto)) (Variables|/Game/Blueprints/ElTosto/BPC_ElTosto.BPC_ElTosto_C|GetFinalScore _asbpc_el_tosto)))))
  (UserInterface|Viewport|AddtoViewport _returnvalue_2 0)
  (Audio|SpawnSoundAttached "/Game/Blueprints/Ending/EndSong.EndSong" (Variables|Collision|GetCapsuleComponent) "None" "0, 0, 0" "0, 0, 0" "KeepRelativeOffset" false 1.0 1.0 0.0 0 0)
  (Variables|/Script/Engine.PlayerController|SetbShowMouseCursor (Game|GetPlayerController 0) true))

(fn ConstructionScript)