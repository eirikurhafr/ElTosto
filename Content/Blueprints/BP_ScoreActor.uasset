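; BP_ScoreActor is a pickup or target actor that awards ScoreToAdd points to the player once, when overlapped or damaged.
; BeginPlay caches the player as BP_Character_ElTosto, retrying the cast every 0.2 seconds until it succeeds.
; Both triggers call GivePlayerScore, which updates the player's score and sets HasGivenScore to block repeat awards.
; Neither trigger checks which actor caused it.
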(event EventBeginPlay
  (bind _asbp_character_el_tosto (Utilities|Casting|CastToBP_Character_ElTosto (Game|GetPlayerCharacter 0) :!label _label)
    (:then
      (Variables|Default|SetPlayer _asbp_character_el_tosto))
    (:CastFailed
      (Utilities|FlowControl|Delay 0.2)
      (goto _label))))

(event Collision|EventActorBeginOverlap
  (params (OtherActor :type Actor%20Object%20Reference))
  (CallFunction|GivePlayerScore))

(event Game|Damage|EventAnyDamage
  (params (Damage :type Float%20%28single-precision%29) (DamageType :type Damage%20Type%20Object%20Reference) (InstigatedBy :type Controller%20Object%20Reference) (DamageCauser :type Actor%20Object%20Reference))
  (CallFunction|GivePlayerScore))

(fn ConstructionScript)

(fn GivePlayerScore
  (if (not (Variables|Default|GetHasGivenScore))
    (Default|UpdateScore (Variables|Default|GetPlayer) (Variables|Default|GetScoreToAdd))
    (Variables|Default|SetHasGivenScore true)))