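; UI manager component that periodically shows random facts with audio on the HUD.
; BeginPlay retries every 0.2 seconds until the HUD is valid, then calls DisplayFact.
; DisplayFact sends a random text and clip to the HUD, plays an attention sound at world origin and reschedules itself.
; The next delay adds random padding to a re-rolled clip's duration, which may differ from the clip sent.
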(event EventBeginPlay
  (Utilities|IsValid (Variables|Default|GetHUD) :!label _label
    (:Is%20Valid
      (Utilities|Time|SetTimerbyFunctionName 0 "DisplayFact" (Math|Random|RandomFloatinRange 1e+01 2e+01))
      (CallFunction|DisplayFact))
    (:Is%20Not%20Valid
      (Utilities|FlowControl|Delay 0.2)
      (goto _label))))

(fn DisplayFact
  (bind _factstrings (Variables|Default|GetFactStrings))
  (bind _factaudio (Variables|Default|GetFactAudio))
  (bind _returnvalue (Utilities|Array|Length _factstrings))
  (bind _returnvalue_2 (- _returnvalue 1))
  (bind _returnvalue_3 (Math|Random|RandomIntegerinRange 0 _returnvalue_2))
  (bind _output (Utilities|Array|Get(acopy) _factaudio _returnvalue_3))
  (Default|DisplayFact (Variables|Default|GetHUD) _output (Utilities|Text|ToText(String) (Utilities|Array|Get(acopy) _factstrings _returnvalue_3)))
  (Audio|PlaySoundatLocation "/Game/SFX/UI/SC_Attention.SC_Attention" "0, 0, 0" "0, 0, 0" 1.0 1.0 0.0 0 0 0)
  (Utilities|Time|SetTimerbyFunctionName 0 "DisplayFact" (+ (Variables|/Script/Engine.SoundBase|GetDuration _output) (Math|Random|RandomFloatinRange 5.0 7.0))))