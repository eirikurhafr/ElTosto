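; ElTosto game state that rate-limits human and crash sound effects.
; PlayHumanSound and PlayCrashSound each spawn a given sound at a location only when their own delay has run out, then reset it to a short cooldown.
; Tick counts both delays down independently, so repeated calls cannot stack sounds of the same category.
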(event EventBeginPlay)

(event EventTick
  (params (DeltaSeconds :type Float%20%28single-precision%29))
  (Utilities|FlowControl|Sequence
    (:then_0
      (if (> (Variables|Default|GetHumanDelay) 0.0)
        (Variables|Default|SetHumanDelay (- (Variables|Default|GetHumanDelay) DeltaSeconds))))
    (:then_1
      (if (> (Variables|Default|GetCrashDelay) 0.0)
        (Variables|Default|SetCrashDelay (- (Variables|Default|GetCrashDelay) DeltaSeconds))))))

(fn ConstructionScript)

(fn PlayHumanSound
  (params (Sound :type Sound%20Base%20Object%20Reference) (Location :type Vector))
  (if (<= (Variables|Default|GetHumanDelay) 0.0)
    (Audio|SpawnSoundatLocation Sound Location "0, 0, 0" 1.0 1.0 0.0 0 0)
    (Variables|Default|SetHumanDelay 0.5)))

(fn PlayCrashSound
  (params (Sound :type Sound%20Base%20Object%20Reference) (Location :type Vector))
  (if (<= (Variables|Default|GetCrashDelay) 0.0)
    (Audio|SpawnSoundatLocation Sound Location "0, 0, 0" 1.0 1.0 0.0 0 0)
    (Variables|Default|SetCrashDelay 0.5)))